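; BP_PCGModule is an actor that configures a PCG graph for a modular tile with a floor and four walls, sized from WallSize.
; Its construction script writes vector parameters to the PCG component's graph instance.
; The floor offset and four opposing X/Y wall offsets derive from half WallSize, while floor scale is the ratio of WallSize to FloorSize.
; The event graph holds only unused placeholder events.
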(event EventBeginPlay)

(event Collision|EventActorBeginOverlap
  (params (OtherActor :type Actor%20Object%20Reference)))

(event EventTick
  (params (DeltaSeconds :type Float%20%28single-precision%29)))

(fn ConstructionScript
  (bind _pcg (Variables|Default|GetPCG))
  (bind _wall_size (Variables|Default|GetWall%20Size))
  (bind _wall_size_2 (Variables|Default|GetWall%20Size))
  (bind _returnvalue (/ _wall_size 2.0))
  (bind _returnvalue_2 (/ _wall_size_2 2.0))
  (bind _graphinstance (Variables|/Script/PCG.PCGComponent|GetGraphInstance _pcg))
  (bind _returnvalue_3 (* _returnvalue_2 -1.0))
  (Effects|Components|ParticleSystem|SetVectorParameter _graphinstance "FloorOffset" (Math|Vector|MakeVector (* _returnvalue -1.0) _returnvalue 0.0))
  (Effects|Components|ParticleSystem|SetVectorParameter _graphinstance "FloorScale" (Math|Conversions|ToVector(Float) (/ (Variables|Default|GetWall%20Size) (Variables|Default|GetFloor%20Size))))
  (Effects|Components|ParticleSystem|SetVectorParameter _graphinstance "WallOffset1" (Math|Vector|MakeVector _returnvalue_2 0.0 0.0))
  (Effects|Components|ParticleSystem|SetVectorParameter _graphinstance "WallOffset2" (Math|Vector|MakeVector _returnvalue_3 0.0 0.0))
  (Effects|Components|ParticleSystem|SetVectorParameter _graphinstance "WallOffset3" (Math|Vector|MakeVector 0.0 _returnvalue_2 0.0))
  (Effects|Components|ParticleSystem|SetVectorParameter _graphinstance "WallOffset4" (Math|Vector|MakeVector 0.0 _returnvalue_3 0.0)))