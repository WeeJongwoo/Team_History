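; BP_TopBasement is the base of a spinning top game, serving as the player's camera and running score and game over.
; On BeginPlay it becomes the view target, creates the HUD widget and enables input, so the Rotate axis yaws its SpringArm.
; Score rises every Tick, so it depends on frame rate, and displays divided by ten.
; A BP_SpinningTop overlapping the Box gets SetSlap, which stops scoring and reveals GameOver.
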(event `self.ReceiveBeginPlay`
  (`PlayerController.SetViewTargetWithBlend` (`GameplayStatics.GetPlayerController` 0) self 0.0 "VTBlend_Linear" 0.0 false)
  (bind _returnvalue (`|CreateWidget` "/Game/HanJinHo/Blueprint/NewWidgetBlueprint.NewWidgetBlueprint_C"))
  (bind _output_get (set `self.Widget` _returnvalue))
  (`Widget.SetVisibility` (`/Game/HanJinHo/Blueprint/NewWidgetBlueprint.GameOver` _output_get) "Hidden")
  (`UserWidget.AddToViewport` _output_get 0)
  (`self.EnableInput` (`GameplayStatics.GetPlayerController` 0)))

(event `InputAxis|Rotate on Axis`
  (params (AxisValue :type "Float (single-precision)"))
  (bind (_returnvalue_roll _returnvalue_pitch _returnvalue_yaw) (`KismetMathLibrary.BreakRotator` (`SpringArmComponent.GetTargetRotation` (`self.SpringArm`))))
  (`SceneComponent.K2_SetRelativeRotation` (`self.SpringArm`) (`KismetMathLibrary.MakeRotator` _returnvalue_roll _returnvalue_pitch (+ _returnvalue_yaw (* (`GameplayStatics.GetWorldDeltaSeconds`) (`self.CameraRotateSpeed`) AxisValue))) false false))

(event `self.ReceiveTick`
  (params (DeltaSeconds :type "Float (single-precision)"))
  (if (not (`self.IsSlap`))
    (bind _result (`/Engine/EditorBlueprintResources/StandardMacros.IncrementInt` (`self.Score`))
      (:`  `
        (bind _output_get (set `self.Score` _result))
        (set `TextBlock.Text` (`|FormatText` "Score : {score}" (/ _output_get 10)) (`/Game/HanJinHo/Blueprint/NewWidgetBlueprint.TextBlock_0` (`self.Widget`)))))))

(event `self.Box.OnComponentBeginOverlap`
  (params (OverlappedComponent :type "PrimitiveComponent Object Reference") (OtherActor :type "Actor Object Reference") (OtherComp :type "PrimitiveComponent Object Reference") (OtherBodyIndex :type Integer) (bFromSweep :type Boolean) (SweepResult :type "HitResult Structure (by ref)"))
  (bind _asbp_spinning_top (cast `/Game/HanJinHo/Blueprint/BP_SpinningTop` OtherActor))
  (`/Game/HanJinHo/Blueprint/BP_SpinningTop.Set Slap` _asbp_spinning_top)
  (set `self.IsSlap` true)
  (`Widget.SetVisibility` (`/Game/HanJinHo/Blueprint/NewWidgetBlueprint.GameOver` (`self.Widget`)) "Visible"))

(fn `UserConstructionScript`)