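; Physics-driven spinning top pawn that the player spins up and steadies with left mouse clicks.
; On BeginPlay it stores its start location, applies an initial torque to Top along its up axis and possesses itself with the first player controller.
; Each click adds world-up torque with a clamped tilt multiplier, plus a force opposing the lean, scaled by tilt from the up-vector dot product, and prints that force factor.
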(event `self.ReceiveBeginPlay`
  (bind _returnvalue_location (`KismetMathLibrary.BreakTransform` (`self.GetTransform`)))
  (set `self.BasicPosition` _returnvalue_location)
  (`PrimitiveComponent.AddTorqueInRadians` (`self.Top`) (* (`self.GetActorUpVector`) 1000.0) "None" true)
  (`Controller.Possess` (`GameplayStatics.GetPlayerController` 0) self))

(event `Key|LeftMouseButton`
  (params (Key :type "Key Structure"))
  (bind _returnvalue (- 1.0 (`KismetMathLibrary.Dot_VectorVector` (`KismetMathLibrary.Vector_Up`) (`self.GetActorUpVector`))))
  (bind _returnvalue_2 (* _returnvalue 9.8))
  (:`Pressed`
    (`PrimitiveComponent.AddTorqueInRadians` (`self.Top`) (* (`KismetMathLibrary.Vector_Up`) (`self.SpinPower`) (`KismetMathLibrary.FClamp` (* _returnvalue 250.0) 1.0 10.0)) "None" true)
    (`PrimitiveComponent.AddForce` (`self.Top`) (* (`KismetMathLibrary.Normal` (- (`KismetMathLibrary.Vector_Up`) (`self.GetActorUpVector`))) (`self.ForcePower`) _returnvalue_2) "None" true)
    (`KismetSystemLibrary.PrintText` (`KismetTextLibrary.Conv_DoubleToText` _returnvalue_2 "HalfToEven"))))

(fn `UserConstructionScript`)