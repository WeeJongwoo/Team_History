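; Legacy physics spinning top that the player keeps spinning with left clicks against growing wobble.
; BeginPlay applies an initial spin torque to Top, and each click adds more.
; Tick uses a Delay to roughly once per second push Body in a random horizontal direction and apply counter-torque to Top, both scaling with elapsed time up to clamps.
; SetSlap sets a flag that halts further disturbances and click input.
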(event `self.ReceiveBeginPlay`
  (`PrimitiveComponent.AddTorqueInRadians` (`self.Top`) (* (`KismetMathLibrary.Vector_Up`) (`self.TorquePower`) 2.0) "None" true))

(event `self.ReceiveTick`
  (params (DeltaSeconds :type "Float (single-precision)"))
  (bind _returnvalue (`KismetMathLibrary.FClamp` (`self.TimeRecord`) 1.0 2.5))
  (bind _returnvalue_2 (`KismetMathLibrary.FClamp` (`self.TimeRecord`) 1.0 3.3))
  (if (not (`self.IsSlap`))
    (`KismetSystemLibrary.Delay` 1.0)
    (set `self.TimeRecord` (+ (`self.TimeRecord`) 0.2))
    (switch `int` (`KismetMathLibrary.RandomIntegerInRange` 0 3)
      (:`0`
        (`PrimitiveComponent.AddForce` (`self.Body`) (* (`SceneComponent.GetRightVector` (`self.Body`)) (`self.ResistPower`) 1.0 _returnvalue) "None" true)
        (`KismetSystemLibrary.PrintText` "right"))
      (:`1`
        (`PrimitiveComponent.AddForce` (`self.Body`) (* (`SceneComponent.GetRightVector` (`self.Body`)) (`self.ResistPower`) -1.0 _returnvalue) "None" true)
        (`KismetSystemLibrary.PrintText` "left"))
      (:`2`
        (`PrimitiveComponent.AddForce` (`self.Body`) (* (`SceneComponent.GetForwardVector` (`self.Body`)) (`self.ResistPower`) 1.0 _returnvalue) "None" true)
        (`KismetSystemLibrary.PrintText` "forward"))
      (:`3`
        (`PrimitiveComponent.AddForce` (`self.Body`) (* (`SceneComponent.GetForwardVector` (`self.Body`)) (`self.ResistPower`) -1.0 _returnvalue) "None" true)
        (`KismetSystemLibrary.PrintText` "backward")))
    (`PrimitiveComponent.AddTorqueInRadians` (`self.Top`) (/ (* (`KismetMathLibrary.Vector_Up`) (`self.TorquePower`) -1.0 _returnvalue_2) 5.0) "None" true)
    (`KismetSystemLibrary.PrintText` (`|FormatText` "{time}" _returnvalue_2))))

(event `Key|LeftMouseButton`
  (params (Key :type "Key Structure"))
  (:`Pressed`
    (if (not (`self.IsSlap`))
      (`PrimitiveComponent.AddTorqueInRadians` (`self.Top`) (* (`KismetMathLibrary.Vector_Up`) (`self.TorquePower`)) "None" true))))

(fn `Set Slap`
  (set `self.IsSlap` true))

(fn `UserConstructionScript`)