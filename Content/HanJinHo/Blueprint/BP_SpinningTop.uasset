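; BP_SpinningTop is a physics-driven spinning top pawn that the player controller possesses at BeginPlay.
; BeginPlay records the start location and applies an initial torque to Edge along its up vector.
; Left click torques Edge along a normalized Point-minus-Edge vector, which mixes world and relative locations.
; It also pushes Point along the flattened world-space Edge-to-Point offset scaled by ForcePower, printing that force.
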(event `self.ReceiveBeginPlay`
  (bind _returnvalue_location (`KismetMathLibrary.BreakTransform` (`self.GetTransform`)))
  (bind _edge (`self.Edge`))
  (set `self.BasicPosition` _returnvalue_location)
  (`PrimitiveComponent.AddTorqueInRadians` _edge (* (`SceneComponent.GetUpVector` _edge) 500.0) "None" true)
  (`Controller.Possess` (`GameplayStatics.GetPlayerController` 0) self))

(event `Key|LeftMouseButton`
  (params (Key :type "Key Structure"))
  (bind (_returnvalue_x _returnvalue_y) (`KismetMathLibrary.BreakVector` (- (`SceneComponent.K2_GetComponentLocation` (`self.Point`)) (`SceneComponent.K2_GetComponentLocation` (`self.Edge`)))))
  (bind _returnvalue (* (`KismetMathLibrary.MakeVector` _returnvalue_x _returnvalue_y) (`self.ForcePower`)))
  (:`Pressed`
    (`PrimitiveComponent.AddTorqueInRadians` (`self.Edge`) (* (`KismetMathLibrary.Normal` (- (`SceneComponent.K2_GetComponentLocation` (`self.Point`)) (`SceneComponent.RelativeLocation` (`self.Edge`)))) (`self.SpinPower`)) "None" true)
    (`PrimitiveComponent.AddForce` (`self.Point`) _returnvalue "None" true)
    (`KismetSystemLibrary.PrintText` (`KismetTextLibrary.Conv_VectorToText` _returnvalue))))

(fn `UserConstructionScript`)