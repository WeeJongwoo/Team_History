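; BP_Hand is a VR hand that sets up a left or right Manny XR mesh and matching motion controller source from the LeftHand flag.
; HandleGrab finds a BP_GrabComponent on an actor hit by a debug-drawn sphere trace at the controller, then stores it if TryGrab succeeds.
; HandleRelease calls TryRelease on the held component.
; Both handlers also drive the grasp pose alpha in ABP_Hand, even when nothing is held.
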(event `self.ReceiveBeginPlay`
  (if (`self.bLeftHand`)
    (`SkeletalMeshComponent.SetSkeletalMeshAsset` (`self.HandMesh`) "/Game/Characters/MannequinsXR/Meshes/SKM_MannyXR_left.SKM_MannyXR_left")
    (`SceneComponent.K2_SetRelativeRotation` (`self.HandMesh`) (struct :`Pitch` -90.0 :`Roll` -90.0) false false)
    (set `MotionControllerComponent.MotionSource` "Left" (`self.MotionController`))
    (else
      (`SkeletalMeshComponent.SetSkeletalMeshAsset` (`self.HandMesh`) "/Game/Characters/MannequinsXR/Meshes/SKM_MannyXR_right.SKM_MannyXR_right")
      (`SceneComponent.K2_SetRelativeRotation` (`self.HandMesh`) (struct :`Pitch` 90.0 :`Roll` 90.0) false false)
      (set `MotionControllerComponent.MotionSource` "Right" (`self.MotionController`)))))

(fn `FindGrabComponentNearHand`
  (returns (NewParam :type "/Game/HanJinHo/Blueprint/BP_GrabComponent Object Reference"))
  (locals (LocalGripPosition :type "Vector Structure" :default (0.0 0.0 0.0)) (LocalGrabComponent :type "/Game/HanJinHo/Blueprint/BP_GrabComponent Object Reference"))
  (`|ExecutionSequence`
    (:`then_0`
      (bind _output_get (set `local.LocalGripPosition` (`SceneComponent.K2_GetComponentLocation` (`self.MotionController`))))
      (bind (_outhit _returnvalue) (`KismetSystemLibrary.SphereTraceSingleForObjects` :`Start` _output_get :`End` _output_get :`Radius` (`self.GripRadius`) :`ObjectTypes` (`|MakeArray` "ObjectTypeQuery8" :!type "EObjectTypeQuery Enum") :`DrawDebugType` "ForDuration"))
      (if _returnvalue
        (bind _returnvalue_2 (`self.GetComponentByClass` (`.HitActor` (`GameplayStatics.BreakHitResult` _outhit)) "/Game/HanJinHo/Blueprint/BP_GrabComponent.BP_GrabComponent_C"))
        (`/Engine/EditorBlueprintResources/StandardMacros.IsValid` _returnvalue_2
          (:`Is Valid`
            (set `local.LocalGrabComponent` _returnvalue_2)))))
    (:`then_1`
      (return (`local.LocalGrabComponent`)))))

(fn `HandleGrab`
  (`|ExecutionSequence`
    (:`then_0`
      (bind _newparam (`self.FindGrabComponentNearHand`))
      (`/Engine/EditorBlueprintResources/StandardMacros.IsValid` _newparam
        (:`Is Valid`
          (bind _bsuccess (`/Game/HanJinHo/Blueprint/BP_GrabComponent.TryGrab` _newparam self))
          (if _bsuccess
            (set `self.HeldComponent` _newparam)))))
    (:`then_1`
      (bind _asabp_hand (cast `/Game/HanJinHo/Blueprint/ABP_Hand` (`SkeletalMeshComponent.GetAnimInstance` (`self.HandMesh`))))
      (set `/Game/HanJinHo/Blueprint/ABP_Hand.PoseAlphaGrasp` 1.0 _asabp_hand))))

(fn `HandleRelease`
  (bind _heldcomponent (`self.HeldComponent`))
  (`|ExecutionSequence`
    (:`then_0`
      (`/Engine/EditorBlueprintResources/StandardMacros.IsValid` _heldcomponent
        (:`Is Valid`
          (`/Game/HanJinHo/Blueprint/BP_GrabComponent.TryRelease` _heldcomponent))))
    (:`then_1`
      (bind _asabp_hand (cast `/Game/HanJinHo/Blueprint/ABP_Hand` (`SkeletalMeshComponent.GetAnimInstance` (`self.HandMesh`))))
      (set `/Game/HanJinHo/Blueprint/ABP_Hand.PoseAlphaGrasp` 0.0 _asabp_hand))))

(fn `UserConstructionScript`)