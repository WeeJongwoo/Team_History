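; BP_SpinTop is a physics-driven spinning top that spins up when play begins and again when hit.
; BeginPlay and the Hitted event both apply upward-axis torque to Top, scaled by TorquePower.
; Disconnected logic would apply growing counter-torque while not slapped and push Body in random horizontal directions, but it never runs.
; SetSlap only raises the IsSlap flag that this unused logic checks, and Tick is empty.
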(event `Hitted`
  (`PrimitiveComponent.AddTorqueInRadians` (`self.Top`) (* (`KismetMathLibrary.Vector_Up`) (`self.TorquePower`) 2.0) "None" true)
  (`KismetSystemLibrary.PrintText` "Hit" true true (struct :`G` 0.66 :`B` 1.0 :`A` 1.0) 5.0))

(event `self.ReceiveBeginPlay`
  (`PrimitiveComponent.AddTorqueInRadians` (`self.Top`) (* (`KismetMathLibrary.Vector_Up`) (`self.TorquePower`) 2.0) "None" true))

(event `self.ReceiveTick`
  (params (DeltaSeconds :type "Float (single-precision)")))

(fn `Set Slap`
  (set `self.IsSlap` true))

(fn `UserConstructionScript`)