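; BP_Wallline1 is a spline-driven construction actor that, judging by its name, lays out a line of wall along an editable path.
; Its construction script divides the spline length by MeshSize and adds a scaled spline mesh component for each full segment, skipping any partial remainder.
; Each segment takes local-space positions and tangents from the spline, with tangent length clamped to MeshSize to limit distortion.
; The event graph holds only empty default events.
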(fn `UserConstructionScript`
  (bind _meshsize (`self.MeshSize`))
  (bind _spline (`self.Spline`))
  (bind _spline_2 (`self.Spline`))
  (for _index (range (+ (`KismetMathLibrary.FTrunc` (/ (`SplineComponent.GetSplineLength` (`self.Spline`)) (`self.MeshSize`))) 1))
    (bind _returnvalue (* _index _meshsize))
    (bind _returnvalue_2 (+ _returnvalue _meshsize))
    (if (not (> _returnvalue_2 (`SplineComponent.GetSplineLength` (`self.Spline`))))
      (bind _returnvalue_3 (`AddComponent|NODE_AddSplineMeshComponent-4` :`RelativeTransform` (`KismetMathLibrary.MakeTransform` (0.0 0.0 0.0) (struct) (1.5 1.5 1.5))))
      (`SplineMeshComponent.SetStartAndEnd` _returnvalue_3 (`SplineComponent.GetLocationAtDistanceAlongSpline` _spline_2 _returnvalue "Local") (`KismetMathLibrary.ClampVectorSize` (`SplineComponent.GetTangentAtDistanceAlongSpline` _spline_2 _returnvalue "Local") 0.0 (`self.MeshSize`)) (`SplineComponent.GetLocationAtDistanceAlongSpline` _spline _returnvalue_2 "Local") (`KismetMathLibrary.ClampVectorSize` (`SplineComponent.GetTangentAtDistanceAlongSpline` _spline _returnvalue_2 "Local") 0.0 (`self.MeshSize`)) true))))