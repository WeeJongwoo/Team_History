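; BP_Adv_NPC is an NPC that offers itself for conversation when the player's VR pawn enters its box, and can play body montages.
; PlayBodyMontage blocking-loads the montage asset, then relays it through server and multicast events intended for replicated playback.
; The construction script creates a dynamic female-body material on mesh slot 0, also assigns it to slot 1, and tints it with the Color variable.
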(event `/Game/VRSubtitle/Blueprints/BI_AdvancedDialogue.Play Body Montage`
  (params (`Body Montage` :type "AnimMontage Soft Object Reference"))
  ;[1 1 1] Play Body Montage REPLICATED
  (bind _returnvalue (`KismetSystemLibrary.LoadAsset_Blocking` `Body Montage`))
  (`self.Server Body Montage` (`self.Mesh`) (cast `AnimMontage` _returnvalue :!pure true)))

(event `Server Body Montage`
  (params (InSkeletalMeshComponent :type "SkeletalMeshComponent Object Reference") (MontageToPlay :type "AnimMontage Object Reference"))
  ;[1 1 1] Play Body Montage REPLICATED
  (`self.Multicast Body Montage` InSkeletalMeshComponent MontageToPlay))

(event `Multicast Body Montage`
  (params (InSkeletalMeshComponent :type "SkeletalMeshComponent Object Reference") (MontageToPlay :type "AnimMontage Object Reference"))
  ;[1 1 1] Play Body Montage REPLICATED
  (`|PlayMontage` InSkeletalMeshComponent MontageToPlay))

(event `self.Box.OnComponentBeginOverlap`
  (params (OverlappedComponent :type "PrimitiveComponent Object Reference") (OtherActor :type "Actor Object Reference") (OtherComp :type "PrimitiveComponent Object Reference") (OtherBodyIndex :type Integer) (bFromSweep :type Boolean) (SweepResult :type "HitResult Structure (by ref)"))
  (if (== OtherActor (`GameplayStatics.GetPlayerPawn` 0))
    (bind _asvrpawn (cast `/Game/VRTemplate/Blueprints/VRPawn` OtherActor))
    (message `/Game/VRSubtitle/Blueprints/BI_VR_Dialogue_Interface.Set Talkable` _asvrpawn self true)))

(fn `UserConstructionScript`
  (bind _mesh (`self.Mesh`))
  (bind _returnvalue (`PrimitiveComponent.CreateDynamicMaterialInstance` _mesh 0 "/Game/VRSubtitle/Demo/Mannequin/Character/Materials/MI_Female_Body.MI_Female_Body" "None"))
  (`PrimitiveComponent.SetMaterial` _mesh 1 _returnvalue)
  (`MaterialInstanceDynamic.SetVectorParameterValue` _returnvalue "Color" (`self.Color`)))