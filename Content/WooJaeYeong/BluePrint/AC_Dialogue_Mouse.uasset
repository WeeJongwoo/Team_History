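; Dialogue component for the Mouse NPC, a guide that offers in Korean to lead the player.
; It overrides Dialogue, branching on the tree index and each chosen option through AddDialogue nodes.
; Accepting guidance switches to tree index 1, where later talks show one of two random "follow me" lines.
; It halts the first CNPCMovementPath actor found via CanMoveNPC during conversation and releases it when each branch ends.
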(fn `Dialogue`
  (bind _returnvalue (`GameplayStatics.GetActorOfClass` "/Script/History.CNPCMovementPath"))
  (set `self.AINPC` _returnvalue)
  (`parent.Dialogue`)
  (switch `int` (`self.DialogueTreeIndex`)
    (:`0`
      (bind (_state _optionindex) (`self.AddDialogue` "Mouse" "반가워요 뭐 필요하신가요?" (`|MakeArray` "네" "아니요" :!type "Text")))
      (set `CNPCMovementPath.bCanMoveNPC` false (`self.AINPC`))
      (switch `/Game/WooJaeYeong/BluePrint/Enum_DialogueState` _state
        (:`NewEnumerator0`
          (switch `int` _optionindex
            (:`0`
              ;[1 1 1] 대화 속
              (bind (_state_2 _optionindex_2) (`self.AddDialogue` "Mouse" "무엇이 필요하죠?" (`|MakeArray` "안내" "괜찮아요" :!type "Text")))
              (switch `/Game/WooJaeYeong/BluePrint/Enum_DialogueState` _state_2
                (:`NewEnumerator0`
                  (switch `int` _optionindex_2
                    (:`0`
                      (bind _state_3 (`self.AddDialogue` "Mouse" "안내해드릴게요 따라와요" (`|MakeArray` "네" :!type "Text")))
                      (switch `/Game/WooJaeYeong/BluePrint/Enum_DialogueState` _state_3
                        (:`NewEnumerator0`
                          (`self.SetDialogTreeIndex` 1)
                          (`self.ClearDialogueProgress`)
                          (set `CNPCMovementPath.bCanMoveNPC` true (`self.AINPC`)))))
                    (:`1`
                      (bind _state_4 (`self.AddDialogue` "Mouse" "알겠습니다" (`|MakeArray` "계속" :!type "Text")))
                      (switch `/Game/WooJaeYeong/BluePrint/Enum_DialogueState` _state_4
                        (:`NewEnumerator0`
                          (`self.RemoveDialogueProgress` 0)
                          (`self.ClearDialogueProgress`)
                          (set `CNPCMovementPath.bCanMoveNPC` true (`self.AINPC`)))))))))
            (:`1`
              ;[1 1 1] 대화 끝
              (bind _state_5 (`self.AddDialogue` "Mouse" "아 알겠습니다" (`|MakeArray` "계속" :!type "Text")))
              (switch `/Game/WooJaeYeong/BluePrint/Enum_DialogueState` _state_5
                (:`NewEnumerator0`
                  (`self.ClearDialogueProgress`)
                  (`self.CloseConversation`)
                  (set `CNPCMovementPath.bCanMoveNPC` true (`self.AINPC`)))))))))
    (:`1`
      (set `CNPCMovementPath.bCanMoveNPC` false (`self.AINPC`))
      (bind _state_6 (`self.AddDialogue` "Mouse" (select `int` (`KismetMathLibrary.RandomIntegerInRange` 0 1) :`0` "따라오세요" :`1` "따라오셈요" :!type "Text") (`|MakeArray` "계속" :!type "Text")))
      (switch `/Game/WooJaeYeong/BluePrint/Enum_DialogueState` _state_6
        (:`NewEnumerator0`
          (`self.ClearDialogueProgress`)
          (`self.CloseConversation`)
          (set `CNPCMovementPath.bCanMoveNPC` true (`self.AINPC`)))))))