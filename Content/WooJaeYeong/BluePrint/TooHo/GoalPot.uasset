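; GoalPot is the goal actor for a TooHo arrow-into-pot minigame, counting arrows that enter it.
; On BeginPlay it creates the W_TooHo widget for the first player and adds it to the viewport.
; When Box3 is overlapped by the Arrow actor returned by GetActorOfClass, it prints that actor's name and increments Score.
; The graph never pushes Score to the widget, as its GetScoreText call is unconnected.
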(event `self.ReceiveBeginPlay`
  (bind _returnvalue (`|CreateWidget` "/Game/WooJaeYeong/UI/W_TooHo.W_TooHo_C" (`GameplayStatics.GetPlayerController` 0)))
  (`UserWidget.AddToViewport` _returnvalue 0))

(event `self.Box3.OnComponentBeginOverlap`
  (params (OverlappedComponent :type "PrimitiveComponent Object Reference") (OtherActor :type "Actor Object Reference") (OtherComp :type "PrimitiveComponent Object Reference") (OtherBodyIndex :type Integer) (bFromSweep :type Boolean) (SweepResult :type "HitResult Structure (by ref)"))
  (bind _returnvalue (`GameplayStatics.GetActorOfClass` "/Game/WooJaeYeong/BluePrint/TooHo/Arrow.Arrow_C"))
  (bind _output_get (set `self.Arrow` _returnvalue))
  (if (== OtherActor _output_get)
    (`KismetSystemLibrary.PrintText` (`|FormatText` (`KismetTextLibrary.Conv_StringToText` (`KismetSystemLibrary.GetObjectName` OtherActor))))
    (`/Engine/EditorBlueprintResources/StandardMacros.IncrementInt` (`self.Score`))))

(fn `UserConstructionScript`)