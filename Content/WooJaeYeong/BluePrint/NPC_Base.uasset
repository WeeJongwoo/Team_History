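; Base NPC Blueprint for interactable characters that display a name and take part in conversations.
; The construction script writes CharacterName into the TxtCharacterName component.
; SetInteractableState shows or hides that name according to whether interaction is available.
; ConversationClose forwards the end of a conversation to InteractInstigator through its ConversationCloseMessage call.
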(event `/Game/WooJaeYeong/BluePrint/BPI_Interactable.SetInteractableState`
  (params (bCanShowInteract :type Boolean))
  (if bCanShowInteract
    (`SceneComponent.SetVisibility` (`self.Txt_CharacterName`) true false)
    (else
      (`SceneComponent.SetVisibility` (`self.Txt_CharacterName`) false false))))

(event `/Game/WooJaeYeong/BluePrint/BPI_Interactable.ConversationClose`
  (message `/Game/WooJaeYeong/BluePrint/BPI_Interactable.ConversationClose` (`self.InteractInstigator`)))

(fn `UserConstructionScript`
  (`TextRenderComponent.K2_SetText` (`self.Txt_CharacterName`) (`self.CharacterName`)))